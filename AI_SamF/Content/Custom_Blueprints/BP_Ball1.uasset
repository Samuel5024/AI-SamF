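; BP_Ball1 is a blue collectible ball that a character picks up by interacting with it.
; On Interact, it increments the valid character's BallCount, grows that character's scale by five percent, then destroys itself.
; The Construction Script applies the solid blue material to its Sphere component.
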(event EventInteract
  (params (Character :type BP%20Third%20Person%20Character%20Object%20Reference))
  (Utilities|IsValid Character
    (:Is%20Valid
      (Variables|/Game/ThirdPerson/Blueprints/Blueprints/BP_ThirdPersonCharacter.BP_ThirdPersonCharacter_C|SetBall_Count Character (+ (Variables|/Game/ThirdPerson/Blueprints/Blueprints/BP_ThirdPersonCharacter.BP_ThirdPersonCharacter_C|GetBall_Count Character) 1))
      (Transformation|SetActorScale3D Character (* (Transformation|GetActorScale3D Character) "1.050000,1.050000,1.050000"))
      (Actor|DestroyActor))))

(fn ConstructionScript
  (Rendering|Material|SetMaterial (Variables|Default|GetSphere) 0 "/Game/LevelPrototyping/Materials/MI_Solid_Blue.MI_Solid_Blue"))