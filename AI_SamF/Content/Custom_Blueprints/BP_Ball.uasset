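; BP_Ball is a collectible ball that the third-person player character picks up on contact.
; Construction gives the sphere a solid blue material, which BeginPlay swaps for CE_OpaqueReference after caching the player character.
; When that character overlaps the box, the ball increments the character's BallCount, shrinks the character by a fixed factor and destroys itself.
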(event OnComponentBeginOverlap(Box)
  (params (OverlappedComponent :type Primitive%20Component%20Object%20Reference) (OtherActor :type Actor%20Object%20Reference) (OtherComp :type Primitive%20Component%20Object%20Reference) (OtherBodyIndex :type Integer) (bFromSweep :type Boolean) (SweepResult :type Hit%20Result%20Structure%20%28by%20ref%29))
  (bind _as_bp_third_person_character (Variables|Default|GetAs%20BP%20Third%20Person%20Character))
  (if (== OtherActor (Variables|Default|GetAs%20BP%20Third%20Person%20Character))
    (CallFunction|BallCount)
    (Transformation|SetActorScale3D _as_bp_third_person_character (* (Transformation|GetActorScale3D _as_bp_third_person_character) "0.900000,0.900000,0.900000"))
    (Actor|DestroyActor)))

(event EventBeginPlay
  (bind _asbp_third_person_character (Utilities|Casting|CastToBP_ThirdPersonCharacter (Game|Player|GetPlayerPawn 0)))
  (Variables|Default|SetAs%20BP%20Third%20Person%20Character _asbp_third_person_character)
  (Rendering|Material|SetMaterial (Variables|Default|GetSphere) 0 "/DatasmithContent/Materials/CE_OpaqueReference.CE_OpaqueReference"))

(fn ConstructionScript
  (Rendering|Material|SetMaterial (Variables|Default|GetSphere) 0 "/Game/LevelPrototyping/Materials/MI_Solid_Blue.MI_Solid_Blue"))

(fn BallCount
  (bind _as_bp_third_person_character (Variables|Default|GetAs%20BP%20Third%20Person%20Character))
  (Variables|/Game/ThirdPerson/Blueprints/Blueprints/BP_ThirdPersonCharacter.BP_ThirdPersonCharacter_C|SetBall_Count _as_bp_third_person_character (+ (Variables|/Game/ThirdPerson/Blueprints/Blueprints/BP_ThirdPersonCharacter.BP_ThirdPersonCharacter_C|GetBall_Count _as_bp_third_person_character) 1)))